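; Player controller that forwards Enhanced Input for moving, camera, shooting, aiming and jumping to the possessed BP_Character.
; On local possession of a new character, it rebuilds the player HUD and a toggleable game info HUD.
; Game start adds the input mapping context; game end removes it, clears held character inputs and shows game info.
; Debug keys host a session on the test level or join the first one found.
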(event Custom|OnStartGame
  (Input|AddMappingContext (PlayerController|LocalPlayerSubsystems|GetEnhancedInputLocalPlayerSubsystem) "/Game/MyContent/Player/Inputs/IMC_CharacterControls.IMC_CharacterControls" 0 "(bIgnoreAllPressedKeysUntilRelease=True,bForceImmediately=False,bNotifyUserSettings=False)"))

(event Custom|OnEndGame
  (Input|RemoveMappingContext (PlayerController|LocalPlayerSubsystems|GetEnhancedInputLocalPlayerSubsystem) "/Game/MyContent/Player/Inputs/IMC_CharacterControls.IMC_CharacterControls" "(bIgnoreAllPressedKeysUntilRelease=True,bForceImmediately=False,bNotifyUserSettings=False)")
  (Class|MGDCharacter|PureMoveCharacter (Variables|Default|GetCharRef))
  (Class|MGDCharacter|PureRotateController (Variables|Default|GetCharRef))
  (Default|PullWeaponTrigger (Variables|Default|GetCharRef) false)
  (Default|AimDownSights (Variables|Default|GetCharRef) false)
  (if (not (UserInterface|Viewport|IsinViewport (Variables|Default|GetGameInfoHUD)))
    (UserInterface|Viewport|AddtoPlayerScreen (Variables|Default|GetGameInfoHUD))))

(event Input|EnhancedActionEvents|EnhancedInputActionIA_Move
  (params (ActionValue :type Vector%202D%20Structure) (ElapsedSeconds :type Float%20%28double-precision%29) (TriggeredSeconds :type Float%20%28double-precision%29) (InputAction :type Input%20Action%20Object%20Reference :default "/Game/MyContent/Player/Inputs/IA_Move.IA_Move"))
  (:Triggered
    (Class|MGDCharacter|PureMoveCharacter (Variables|Default|GetCharRef) ActionValue :!label _label))
  (:Canceled
    (goto _label))
  (:Completed
    (goto _label)))

(event Input|EnhancedActionEvents|EnhancedInputActionIA_TurnCamera
  (params (ActionValue :type Vector%202D%20Structure) (ElapsedSeconds :type Float%20%28double-precision%29) (TriggeredSeconds :type Float%20%28double-precision%29) (InputAction :type Input%20Action%20Object%20Reference :default "/Game/MyContent/Player/Inputs/IA_TurnCamera.IA_TurnCamera"))
  (:Triggered
    (Class|MGDCharacter|PureRotateController (Variables|Default|GetCharRef) ActionValue :!label _label))
  (:Canceled
    (goto _label))
  (:Completed
    (goto _label)))

(event Input|EnhancedActionEvents|EnhancedInputActionIA_Shoot
  (params (ActionValue :type Boolean) (ElapsedSeconds :type Float%20%28double-precision%29) (TriggeredSeconds :type Float%20%28double-precision%29) (InputAction :type Input%20Action%20Object%20Reference :default "/Game/MyContent/Player/Inputs/IA_Shoot.IA_Shoot"))
  (Default|PullWeaponTrigger (Variables|Default|GetCharRef) ActionValue))

(event Input|EnhancedActionEvents|EnhancedInputActionIA_Aim
  (params (ActionValue :type Boolean) (ElapsedSeconds :type Float%20%28double-precision%29) (TriggeredSeconds :type Float%20%28double-precision%29) (InputAction :type Input%20Action%20Object%20Reference :default "/Game/MyContent/Player/Inputs/IA_Aim.IA_Aim"))
  (Default|AimDownSights (Variables|Default|GetCharRef) ActionValue))

(event Input|EnhancedActionEvents|EnhancedInputActionIA_GameInfo
  (params (ActionValue :type Boolean) (ElapsedSeconds :type Float%20%28double-precision%29) (TriggeredSeconds :type Float%20%28double-precision%29) (InputAction :type Input%20Action%20Object%20Reference :default "/Game/MyContent/Player/Inputs/IA_GameInfo.IA_GameInfo"))
  (bind _gameinfohud (Variables|Default|GetGameInfoHUD))
  (if (UserInterface|Viewport|IsinViewport (Variables|Default|GetGameInfoHUD))
    (Widget|RemovefromParent _gameinfohud)
    (else
      (UserInterface|Viewport|AddtoPlayerScreen _gameinfohud))))

(event Input|EnhancedActionEvents|EnhancedInputActionIA_Jump
  (params (ActionValue :type Boolean) (ElapsedSeconds :type Float%20%28double-precision%29) (TriggeredSeconds :type Float%20%28double-precision%29) (InputAction :type Input%20Action%20Object%20Reference :default "/Game/MyContent/Player/Inputs/IA_Jump.IA_Jump"))
  (Character|Jump (Variables|Default|GetCharRef)))

(event EventPureonRepPossess
  (params (PossessedPawn :type Pawn%20Object%20Reference))
  (if (Pawn|IsLocalPlayerController)
    (if (!= PossessedPawn (Variables|Default|GetCharRef))
      (Viewport|RemoveAllWidgets)
      (bind _asbp_character (Utilities|Casting|CastToBP_Character PossessedPawn))
      (Variables|Default|SetCharRef _asbp_character)
      (bind _returnvalue (UserInterface|CreateWidget "/Game/MyContent/Player/BP_UI_PlayerHUD.BP_UI_PlayerHUD_C" self))
      (bind _output_get (Variables|Default|SetPlayerHUD _returnvalue))
      (UserInterface|Viewport|AddtoPlayerScreen _output_get)
      (bind _returnvalue_2 (UserInterface|CreateWidget "/Game/MyContent/Player/BP_UI_GameInfoHUD.BP_UI_GameInfoHUD_C" self))
      (Variables|Default|SetGameInfoHUD _returnvalue_2))))

(event Input|KeyboardEvents|DebugKey1
  (params (Key :type Key%20Structure :default "None") (ActionValue :type Input%20Action%20Value%20Structure))
  ;[1 1 1] Host A Session
  (:Pressed
    (Development|PrintString "Creating session...")
    (|Session self 4 false true
      (:OnSuccess
        (Development|PrintString "Successfully created session" true true "(R=0.000000,G=1.000000,B=0.000000,A=1.000000)")
        (Game|OpenLevel(byObjectReference) "/Game/MyContent/Maps/Lvl_Test.Lvl_Test" true "?listen"))
      (:OnFailure
        (Development|PrintString "Failed to create session" true true "(R=1.000000,G=0.000000,B=0.000000,A=1.000000)")))))

(event Input|KeyboardEvents|DebugKey2
  (params (Key :type Key%20Structure :default "None") (ActionValue :type Input%20Action%20Value%20Structure))
  ;[1 1 1] Join A Session
  (:Pressed
    (Development|PrintString "Finding Sessions")
    (bind _results (|FindSessions self 10 false)
      (:OnSuccess
        (Development|PrintString "Found session... trying to join")
        (|JoinSession self (Utilities|Array|Get(acopy) _results)
          (:OnSuccess
            (Development|PrintString "Successfully joined session" true true "(R=0.000000,G=1.000000,B=0.000000,A=1.000000)"))
          (:OnFailure
            (Development|PrintString "Failed to join session" true true "(R=1.000000,G=0.000000,B=0.000000,A=1.000000)"))))
      (:OnFailure
        (Development|PrintString "Failed to find a session" true true "(R=1.000000,G=0.000000,B=0.000000,A=1.000000)")))))

(fn ConstructionScript)