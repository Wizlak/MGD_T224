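; Sniper rifle pickup that gives the character a weapon and enables its sniper state.
; On overlap with a BP_Character, it sets the aim zoom value and flags HasSniper directly.
; Separately, the Pickup function activates the weapon class from a valid WeaponAsset, then calls the Multi_SniperSound event to play a 2D reload cue.
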(event Custom|Multi_SniperSound
  (Audio|PlaySound2D "/Game/MilitaryWeapDark/Sound/Rifle/Rifle_ReloadInsert_Cue.Rifle_ReloadInsert_Cue" 1.0 1.0 0.0 0 0))

(event Collision|EventActorBeginOverlap
  (params (OtherActor :type Actor%20Object%20Reference))
  (bind _asbp_character (Utilities|Casting|CastToBP_Character OtherActor))
  (Variables|/Game/MyContent/Characters/BP_Character.BP_Character_C|SetZoomAim _asbp_character -1e+03)
  (Variables|/Game/MyContent/Characters/BP_Character.BP_Character_C|SetHasSniper _asbp_character true))

(fn ConstructionScript
  (|CallParentFunction))

(fn Pickup
  (params (Character :type BP%20Character%20Object%20Reference))
  (bind _weaponasset (Variables|Default|GetWeaponAsset)
    (:then
      (Default|ActivateWeapon Character (Variables|/Game/MyContent/Pickups/BP_DA_WeaponPickup.BP_DA_WeaponPickup_C|GetWeaponClass _weaponasset))
      (CallFunction|MultiSniperSound))
    (:else)))