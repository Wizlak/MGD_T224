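; Base pickup actor that spins while active and is collected when a BP_Character overlaps its detection capsule.
; On authority, the overlap calls the empty Pickup hook, then a multicast-named event deactivates it and the server starts a reactivation timer.
; Deactivate and Reactivate toggle the active flag and decal glow through a dynamic material, then call empty OnDeactivate and OnReactivate hooks.
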(event OnComponentBeginOverlap(DetectionCapsule)
  (params (OverlappedComponent :type Primitive%20Component%20Object%20Reference) (OtherActor :type Actor%20Object%20Reference) (OtherComp :type Primitive%20Component%20Object%20Reference) (OtherBodyIndex :type Integer) (bFromSweep :type Boolean) (SweepResult :type Hit%20Result%20Structure%20%28by%20ref%29))
  (if (Variables|Default|GetIsActive)
    (bind _asbp_character (Utilities|Casting|CastToBP_Character OtherActor))
    (Networking|SwitchHasAuthority
      (:Authority
        (CallFunction|Pickup _asbp_character)
        (CallFunction|MultiDeactivate)))))

(event Custom|Multi_Deactivate
  (CallFunction|Deactivate))

(event Custom|Multi_Reactivate
  (CallFunction|Reactivate))

(event EventTick
  (params (DeltaSeconds :type Float%20%28single-precision%29))
  (if (Variables|Default|GetIsActive)
    (Transformation|AddRelativeRotation (Variables|Default|GetMeshTransform) (Math|Rotator|MakeRotator 0.0 0.0 (* DeltaSeconds 8e+01)) false false)))

(event EventBeginPlay
  (bind _returnvalue (Rendering|Material|CreateDynamicMaterialInstance (Variables|Default|GetDecal) :!class /Script/Engine.DecalComponent))
  (Variables|Default|SetDecalMaterial _returnvalue)
  (CallFunction|Reactivate))

(fn ConstructionScript)

(fn Pickup
  (params (Character :type BP%20Character%20Object%20Reference)))

(fn Deactivate
  (Variables|Default|SetIsActive false)
  (Utilities|FlowControl|Sequence
    (:then_0
      (Networking|SwitchHasAuthority
        (:Authority
          (bind _returnvalue (Utilities|Time|SetTimerbyEvent (EventDispatchers|CreateEvent :!event Custom|Multi_Reactivate) (Variables|Default|GetReactivateTime)))
          (Variables|Default|SetTH_Reactivate _returnvalue))))
    (:then_1
      (Rendering|Material|SetScalarParameterValue (Variables|Default|GetDecalMaterial) "Emissive Power" 0.0 :!class /Script/Engine.MaterialInstanceDynamic)
      (CallFunction|OnDeactivate))))

(fn OnDeactivate)

(fn OnReactivate)

(fn Reactivate
  (Variables|Default|SetIsActive true)
  (Rendering|Material|SetScalarParameterValue (Variables|Default|GetDecalMaterial) "Emissive Power" 5e+01 :!class /Script/Engine.MaterialInstanceDynamic)
  (CallFunction|OnReactivate))