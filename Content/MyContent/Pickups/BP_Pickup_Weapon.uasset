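; Weapon pickup that gives the character the weapon class defined in its WeaponAsset.
; Construction sets the skeletal mesh from that asset; Pickup activates the weapon and triggers a multi-named reload-sound event that plays in 2D.
; Deactivate and reactivate overrides extend the parent pickup by hiding and showing the mesh.
; Separately, any BP_Character overlap sets ZoomAim and clears the HasSniper flag, independent of the pickup logic.
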(event Custom|Multi_WeaponSound
  (Audio|PlaySound2D "/Game/MilitaryWeapDark/Sound/Rifle/Rifle_ReloadInsert_Cue.Rifle_ReloadInsert_Cue" 1.0 1.0 0.0 0 0))

(event Collision|EventActorBeginOverlap
  (params (OtherActor :type Actor%20Object%20Reference))
  (bind _asbp_character (Utilities|Casting|CastToBP_Character OtherActor))
  (Variables|/Game/MyContent/Characters/BP_Character.BP_Character_C|SetZoomAim _asbp_character 1.5e+02)
  (Variables|/Game/MyContent/Characters/BP_Character.BP_Character_C|SetHasSniper _asbp_character false))

(fn ConstructionScript
  (|CallParentFunction)
  (bind _weaponasset (Variables|Default|GetWeaponAsset)
    (:then
      (Components|SkeletalMesh|SetSkeletalMeshAsset (Variables|Default|GetSkeletalMesh) (Variables|/Game/MyContent/Pickups/BP_DA_WeaponPickup.BP_DA_WeaponPickup_C|GetSkeletalMesh _weaponasset)))
    (:else)))

(fn Pickup
  (params (Character :type BP%20Character%20Object%20Reference))
  (bind _weaponasset (Variables|Default|GetWeaponAsset)
    (:then
      (Default|ActivateWeapon Character (Variables|/Game/MyContent/Pickups/BP_DA_WeaponPickup.BP_DA_WeaponPickup_C|GetWeaponClass _weaponasset))
      (CallFunction|MultiWeaponSound))
    (:else)))

(fn OnDeactivate
  (|CallParentFunction)
  (Rendering|SetVisibility (Variables|Default|GetSkeletalMesh) false false))

(fn OnReactivate
  (|CallParentFunction)
  (Rendering|SetVisibility (Variables|Default|GetSkeletalMesh) true false))