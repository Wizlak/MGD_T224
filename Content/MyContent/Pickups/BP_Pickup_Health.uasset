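; Health pickup Blueprint, built on a parent pickup class, that restores health to the collecting character.
; Pickup adds a fixed amount to the character's Health without clamping, then calls the Multi_HealthSound event to play a 2D sound cue.
; OnDeactivate and OnReactivate extend the parent's behavior by hiding and showing the two static meshes.
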(event Custom|Multi_HealthSound
  (Audio|PlaySound2D "/Game/MilitaryWeapDark/Sound/Knife/Knife_Raise_Cue.Knife_Raise_Cue" 1.0 1.0 0.0 0 0))

(fn ConstructionScript
  (|CallParentFunction))

(fn Pickup
  (params (Character :type BP%20Character%20Object%20Reference))
  (Variables|/Game/MyContent/Characters/BP_Character.BP_Character_C|SetHealth Character (+ (Variables|/Game/MyContent/Characters/BP_Character.BP_Character_C|GetHealth Character) 30))
  (CallFunction|MultiHealthSound))

(fn OnDeactivate
  (|CallParentFunction)
  (Rendering|SetVisibility (Variables|Default|GetStaticMesh) false false)
  (Rendering|SetVisibility (Variables|Default|GetStaticMesh1) false false))

(fn OnReactivate
  (|CallParentFunction)
  (Rendering|SetVisibility (Variables|Default|GetStaticMesh) true false)
  (Rendering|SetVisibility (Variables|Default|GetStaticMesh1) true false))