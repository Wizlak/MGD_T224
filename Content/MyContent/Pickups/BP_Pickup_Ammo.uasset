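; Ammo pickup Blueprint that extends a parent pickup class and grants a fixed amount of ammo to the collecting character.
; Its Pickup override adds to the character's Ammo and calls a multicast-named event that plays a rifle reload sound as 2D audio.
; Deactivate and reactivate overrides call the parent logic, then hide or show the static mesh.
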(event Custom|Multi_AmmoSound
  (Audio|PlaySound2D "/Game/MilitaryWeapDark/Sound/Rifle/Rifle_ReloadInsert_Cue.Rifle_ReloadInsert_Cue" 1.0 1.0 0.0 0 0))

(fn ConstructionScript
  (|CallParentFunction))

(fn Pickup
  (params (Character :type BP%20Character%20Object%20Reference))
  (Variables|/Game/MyContent/Characters/BP_Character.BP_Character_C|SetAmmo Character (+ (Variables|/Game/MyContent/Characters/BP_Character.BP_Character_C|GetAmmo Character) 1e+02))
  (CallFunction|MultiAmmoSound))

(fn OnDeactivate
  (|CallParentFunction)
  (Rendering|SetVisibility (Variables|Default|GetStaticMesh) false false))

(fn OnReactivate
  (|CallParentFunction)
  (Rendering|SetVisibility (Variables|Default|GetStaticMesh) true false))