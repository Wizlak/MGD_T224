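; Lobby game mode that keeps the player count stored in BP_GameInstance up to date.
; On BeginPlay, PostLogin and OnLogout, it casts the game instance to BP_GameInstance and sets PlayerCount from the current number of player states.
; It contains no other lobby logic, and its construction script is empty.
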(event EventPostLogin
  (params (NewPlayer :type Player%20Controller%20Object%20Reference))
  (bind _asbp_game_instance (Utilities|Casting|CastToBP_GameInstance (Game|GetGameInstance)))
  (Variables|/Game/MyContent/Core/BP_GameInstance.BP_GameInstance_C|SetPlayerCount _asbp_game_instance (Class|GameplayStatics|GetNumPlayerStates)))

(event EventOnLogout
  (params (ExitingController :type Controller%20Object%20Reference))
  (bind _asbp_game_instance (Utilities|Casting|CastToBP_GameInstance (Game|GetGameInstance)))
  (Variables|/Game/MyContent/Core/BP_GameInstance.BP_GameInstance_C|SetPlayerCount _asbp_game_instance (Class|GameplayStatics|GetNumPlayerStates)))

(event EventBeginPlay
  (bind _asbp_game_instance (Utilities|Casting|CastToBP_GameInstance (Game|GetGameInstance)))
  (Variables|/Game/MyContent/Core/BP_GameInstance.BP_GameInstance_C|SetPlayerCount _asbp_game_instance (Class|GameplayStatics|GetNumPlayerStates)))

(fn ConstructionScript)