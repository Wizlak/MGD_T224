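; GM_Battle is the game mode for a multiplayer kill-limit battle, running match start, respawns and the win check.
; PostLogin names players by count and, once the game instance's player count is reached, starts a delayed 3-2-1 countdown before notifying every player state.
; ResetPlayer respawns pawns while the match runs.
; TryWinGame ends it at the kill target, notifying player states and restarting after a short delay.
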(event Custom|BeginGame
  (Utilities|FlowControl|Sequence
    (:then_0
      (Development|PrintString "3" true true "(R=1.000000,G=0.841652,B=0.000000,A=1.000000)"))
    (:then_1
      (Utilities|FlowControl|Delay 1.0)
      (Development|PrintString "2" true true "(R=1.000000,G=0.841652,B=0.000000,A=1.000000)"))
    (:then_2
      (Utilities|FlowControl|Delay 2.0)
      (Development|PrintString "1" true true "(R=1.000000,G=0.841652,B=0.000000,A=1.000000)"))
    (:then_3
      (Utilities|FlowControl|Delay 3.0)
      (Development|PrintString "FIGHT!!!" true true "(R=1.000000,G=0.002520,B=0.000000,A=1.000000)")
      (Variables|Default|SetGameEnded false)
      (for _array_element (Variables|/Script/Engine.GameStateBase|GetPlayerArray (Game|GetGameState))
        (bind _asbp_player_state (Utilities|Casting|CastToBP_PlayerState _array_element))
        (Default|OnStartGame _asbp_player_state)))))

(event Custom|EndGame
  (Variables|Default|SetGameEnded true)
  (for _array_element (Variables|/Script/Engine.GameStateBase|GetPlayerArray (Game|GetGameState))
    (bind _asbp_player_state (Utilities|Casting|CastToBP_PlayerState _array_element))
    (Default|OnEndGame _asbp_player_state))
  (Utilities|FlowControl|Delay 3.0)
  (Class|GameMode|RestartGame))

(event EventPostLogin
  (params (NewPlayer :type Player%20Controller%20Object%20Reference))
  (bind _asbp_player_state (Utilities|Casting|CastToBP_PlayerState (Variables|/Script/Engine.Controller|GetPlayerState NewPlayer)))
  (Default|SetPlayerName _asbp_player_state (Utilities|String|Append "Player " (Utilities|String|ToString(Integer) (Class|GameplayStatics|GetNumPlayerStates))))
  (bind _asbp_game_instance (Utilities|Casting|CastToBP_GameInstance (Game|GetGameInstance)))
  (if (== (Class|GameplayStatics|GetNumPlayerStates) (Variables|/Game/MyContent/Core/BP_GameInstance.BP_GameInstance_C|GetPlayerCount _asbp_game_instance))
    (CallFunction|BeginGame)))

(fn ConstructionScript)

(fn ResetPlayer
  (params (PlayerController :type Player%20Controller%20Object%20Reference))
  (if (not (Variables|Default|GetGameEnded))
    (Actor|DestroyActor (Pawn|GetControlledPawn PlayerController))
    (Class|GameModeBase|RestartPlayer PlayerController)))

(fn TryWinGame
  (params (Kills :type Integer))
  (if (and (>= Kills (Variables|Default|GetKillWinCondition)) (not (Variables|Default|GetGameEnded)))
    (CallFunction|EndGame)))